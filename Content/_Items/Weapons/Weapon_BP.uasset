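; Weapon_BP is a weapon item Blueprint that loads its stats from a data table and shows its name on a pick-up widget.
; On BeginPlay it runs the parent logic, then InitWeaponStats fills WeaponStats from the WeaponData row matching RowName.
; UpdatePickUpText writes that name into the W_ItemPickUp widget, casting and caching it from the PickUpWidget component when not yet valid.
; Interact only forwards to the parent implementation.
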(event `self.ReceiveBeginPlay`
  (`parent.ReceiveBeginPlay`)
  (`self.InitWeaponStats`)
  (`self.UpdatePickUpText`))

(event `InteractInterface.Interact`
  (`parent.Interact`))

(fn `UpdatePickUpText`
  (locals (W_ItemPickUp :type "/Game/_Widgets/W_ItemPickUp Object Reference"))
  (`local.W_ItemPickUp`
    (:`then`
      _)
    (:`else`
      (bind _asw_item_pick_up (cast `/Game/_Widgets/W_ItemPickUp` (`WidgetComponent.GetUserWidgetObject` (`self.PickUpWidget`))))
      (set `local.W_ItemPickUp` _asw_item_pick_up)))
  (`TextBlock.SetText` (`/Game/_Widgets/W_ItemPickUp.ItemName` (`local.W_ItemPickUp`)) (`KismetTextLibrary.Conv_StringToText` (`.Name` (break `WeaponStats` (`self.WeaponStats`))))))

(fn `UserConstructionScript`)