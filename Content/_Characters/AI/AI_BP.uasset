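; AI Blueprint that shows floating damage numbers for hits and damage-over-time ticks.
; Two events create a hit or DOT number widget with crit flags (brutal only for hits), then place it on screen by projecting the hit location through player controller 0.
; Each sets the damage text, passes the widget and world location to StoreHitNumber, defined outside these graphs, and plays the widget's animation.
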(event `self.ShowHitNumber`
  (params (Damage :type Integer) (HitLocation :type "Vector Structure") (bCriticalHit :type Boolean) (bBrutalHit :type Boolean))
  (bind _returnvalue (`|CreateWidget` "/Game/_Widgets/W_HitNumber.W_HitNumber_C" null bCriticalHit bBrutalHit))
  (`UserWidget.AddToViewport` _returnvalue 0)
  (`UserWidget.SetPositionInViewport` _returnvalue (`PlayerController.ProjectWorldLocationToScreen` (`GameplayStatics.GetPlayerController` 0) HitLocation false) true)
  (set `/Game/_Widgets/W_HitNumber.HitNumber` (`KismetTextLibrary.Conv_IntToText` Damage) _returnvalue)
  (`self.StoreHitNumber` _returnvalue HitLocation)
  (`UserWidget.PlayAnimation` _returnvalue (`/Game/_Widgets/W_HitNumber.HitNumberAnmation` _returnvalue) 0.0 1 "Forward" 1.0 false))

(event `self.ShowDOTNumber`
  (params (Damage :type Integer) (HitLocation :type "Vector Structure") (bCriticalHit :type Boolean))
  (bind _returnvalue (`|CreateWidget` "/Game/_Widgets/W_DOTNumber.W_DOTNumber_C" null bCriticalHit))
  (`UserWidget.AddToViewport` _returnvalue 0)
  (`UserWidget.SetPositionInViewport` _returnvalue (`PlayerController.ProjectWorldLocationToScreen` (`GameplayStatics.GetPlayerController` 0) HitLocation false) true)
  (set `/Game/_Widgets/W_DOTNumber.DOTNumber` (`KismetTextLibrary.Conv_IntToText` Damage) _returnvalue)
  (`self.StoreHitNumber` _returnvalue HitLocation)
  (`UserWidget.PlayAnimation` _returnvalue (`/Game/_Widgets/W_DOTNumber.DOTNumberAnmation` _returnvalue) 0.0 1 "Forward" 1.0 false))

(fn `UserConstructionScript`)