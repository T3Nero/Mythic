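; Item Blueprint for a world pickup that shows its name on a pickup widget and can be interacted with.
; On BeginPlay it fills the widget's name text from its ItemInfo, caching the W_ItemPickUp reference from the widget component the first time.
; Interact calls the parent implementation, then hides the widget and disables the pickup collision.
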(event `self.ReceiveBeginPlay`
  (`self.UpdateWidgetDetails`))

(event `InteractInterface.Interact`
  (`parent.Interact`)
  (`SceneComponent.SetVisibility` (`self.PickUpWidget`) false false)
  (`PrimitiveComponent.SetCollisionEnabled` (`self.PickUpCollision`) "NoCollision"))

(fn `UpdateWidgetDetails`
  (locals (W_ItemPickUp :type "/Game/_Widgets/W_ItemPickUp Object Reference"))
  (`local.W_ItemPickUp`
    (:`then`
      _)
    (:`else`
      (bind _asw_item_pick_up (cast `/Game/_Widgets/W_ItemPickUp` (`WidgetComponent.GetUserWidgetObject` (`self.PickUpWidget`))))
      (set `local.W_ItemPickUp` _asw_item_pick_up)))
  (`TextBlock.SetText` (`/Game/_Widgets/W_ItemPickUp.ItemName` (`local.W_ItemPickUp`)) (`KismetTextLibrary.Conv_StringToText` (`.ItemName` (break `ItemInfo` (`self.ItemInfo`))))))

(fn `UserConstructionScript`)