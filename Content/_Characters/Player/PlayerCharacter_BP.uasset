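; Player character Blueprint that implements a directional dodge roll, allowed only while combat state is Unoccupied and not crouching.
; When strafing, the DodgeDiagonally macro checks movement flag pairs for diagonal rolls, with single-direction checks as fallback.
; Non-strafing dodges, or strafing with no direction set, use the forward roll.
; Root-motion montages play slightly slowed, with CombatState held at Dodging until completion restores Unoccupied.
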(event `self.Dodge`
  (if (and (`|EnumEquality` (`self.CombatState`) "ECS_Unoccupied") (not (`self.bCrouching`)))
    (set `self.CombatState` "ECS_Dodging")
    (if (`self.bStrafing`)
      (`self.DodgeDiagonally`
        (:`True`
          _)
        (:`False`
          (if (`self.IsMovingRight`)
            (set `self.DodgeAnimToPlay` "/Game/_Characters/Animations/Dodging/RollRight_Root_Montage.RollRight_Root_Montage")
            (elif (`self.IsMovingLeft`)
              (set `self.DodgeAnimToPlay` "/Game/_Characters/Animations/Dodging/RollLeft_Root_Montage.RollLeft_Root_Montage")
              (elif (`self.IsMovingForward`)
                (set `self.DodgeAnimToPlay` "/Game/_Characters/Animations/Dodging/RollForward_Root_Montage.RollForward_Root_Montage")
                (elif (`self.IsMovingBackward`)
                  (set `self.DodgeAnimToPlay` "/Game/_Characters/Animations/Dodging/RollBackward_Root_Montage.RollBackward_Root_Montage")
                  (else
                    (set `self.DodgeAnimToPlay` "/Game/_Characters/Animations/Dodging/RollForward_Root_Montage.RollForward_Root_Montage" :!label _label))))))))
      (else
        (goto _label)))
    (`|PlayMontage` (`self.Mesh`) (`self.DodgeAnimToPlay`) 0.8
      (:`OnCompleted`
        (set `self.CombatState` "ECS_Unoccupied")))))

(fn `UserConstructionScript`)